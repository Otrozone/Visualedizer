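; Blueprint function library of DMX helpers that push RGB colors to fixtures and LED strips.
; DmxSend fills one segment of a patch's first-mode channel span with a color, cycling R, G, B by channel index, and outputs to hardcoded universe 1.
; DmxSendLedStrip outputs each strip's own channel map to its patch's universe.
; DmxSendLedStripStart triggers DmxSendStart on each strip.
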(fn DmxSend
  (params (FixturePatch :type DMX%20Entity%20Fixture%20Patch%20Object%20Reference) (Color :type Color%20Structure) (SegmentCount :type Integer) (SegmentIndex :type Integer))
  (bind (_b _g _r) (Math|Color|BreakColor Color))
  (bind _channelvalmap (LocalVariables|GetChannelValMap))
  (bind _parentfixturetypetemplate (Variables|/Script/DMXRuntime.DMXEntityFixturePatch|GetParentFixtureTypeTemplate FixturePatch))
  (bind _modes (Variables|/Script/DMXRuntime.DMXEntityFixtureType|GetModes _parentfixturetypetemplate))
  (bind _output (Utilities|Array|Get(acopy) _modes))
  (bind _channelspan (Utilities|Struct|BreakDMXFixtureMode _output))
  (bind _returnvalue (/ _channelspan SegmentCount))
  (for _index (range (* _returnvalue SegmentIndex) (* _returnvalue (+ SegmentIndex 1)))
    (if (== (Math|Integer|%(Integer) _index 3) 0)
      (LocalVariables|SetChannelVal _r)
      (Utilities|Map|Add _channelvalmap _index (LocalVariables|GetChannelVal) :!label _label)
      (elif (== (Math|Integer|%(Integer) _index 3) 1)
        (LocalVariables|SetChannelVal _g)
        (goto _label)
        (elif (== (Math|Integer|%(Integer) _index 3) 2)
          (LocalVariables|SetChannelVal _b)
          (goto _label)))))
  (Class|DMXSubsystem|SendDMXtoOutputPort :ChannelToValueMap _channelvalmap)
  (Development|PrintString 0 "DMX data sent"))

(fn DmxSendLedStrip
  (params (LedStripArray :type Array%20of%20Led%20Strip%20Object%20References))
  (for _array_element LedStripArray
    (bind _channelmap (Default|GetChannelMap _array_element))
    (Class|DMXSubsystem|SendDMXtoOutputPort :ChannelToValueMap _channelmap :LocalUniverse (Variables|/Script/DMXRuntime.DMXEntityFixturePatch|GetUniverseID (Class|DMXEntityReferenceConversions|ToObj(FixturePatchRef) (Variables|/Game/Blueprints/LedStrip.LedStrip_C|GetFixturePatch _array_element))))))

(fn DmxSendLedStripStart
  (params (LedStripArray :type Array%20of%20Led%20Strip%20Object%20References) (__WorldContext :type Object%20Object%20Reference))
  (for _array_element LedStripArray
    (Default|DmxSendStart _array_element)))