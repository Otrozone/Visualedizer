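; Static pawn that lets the player drive RGB DMX lighting through Enhanced Input, adding its mapping context on BeginPlay.
; Red, green and blue actions set each color component to full while held.
; A control action sends the mixed color when pressed and a default color to switch off when released or canceled.
; DmxSendFullColor repeats RGB across a segment of the fixture's first-mode channel span, then outputs it on local universe 1.
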(event Input|EnhancedActionEvents|EnhancedInputActionIA_DmxColorBlue
  (params (ActionValue :type Boolean) (ElapsedSeconds :type Float%20%28double-precision%29) (TriggeredSeconds :type Float%20%28double-precision%29) (InputAction :type Input%20Action%20Object%20Reference :default "/Game/Input/IA_DmxColorBlue.IA_DmxColorBlue"))
  (:Started
    (Development|PrintString "Blue on")
    (Variables|Default|SetColorBlue 255))
  (:Completed
    (Development|PrintString "Blue off")
    (Variables|Default|SetColorBlue 0)))

(event Input|EnhancedActionEvents|EnhancedInputActionIA_DmxColorRed
  (params (ActionValue :type Boolean) (ElapsedSeconds :type Float%20%28double-precision%29) (TriggeredSeconds :type Float%20%28double-precision%29) (InputAction :type Input%20Action%20Object%20Reference :default "/Game/Input/IA_DmxColorRed.IA_DmxColorRed"))
  (:Started
    (Development|PrintString "Red on")
    (Variables|Default|SetColorRed 255))
  (:Completed
    (Development|PrintString "Red off")
    (Variables|Default|SetColorRed 0)))

(event Input|EnhancedActionEvents|EnhancedInputActionIA_DmxColorGreen
  (params (ActionValue :type Boolean) (ElapsedSeconds :type Float%20%28double-precision%29) (TriggeredSeconds :type Float%20%28double-precision%29) (InputAction :type Input%20Action%20Object%20Reference :default "/Game/Input/IA_DmxColorGreen.IA_DmxColorGreen"))
  (:Started
    (Development|PrintString "Green on")
    (Variables|Default|SetColorGreen 255))
  (:Completed
    (Development|PrintString "Green off")
    (Variables|Default|SetColorGreen 0)))

(event Input|EnhancedActionEvents|EnhancedInputActionIA_DmxControlFurnitureFull
  (params (ActionValue :type Boolean) (ElapsedSeconds :type Float%20%28double-precision%29) (TriggeredSeconds :type Float%20%28double-precision%29) (InputAction :type Input%20Action%20Object%20Reference :default "/Game/Input/IA_DmxControlFurnitureFull.IA_DmxControlFurnitureFull"))
  (bind _outfixturepatch (|GetDMXFixturePatch "(DMXLibrary=\"/Script/DMXRuntime.DMXLibrary'/Game/Dmx/LedStripFurniture.LedStripFurniture'\",bDisplayLibraryPicker=True,EntityType=\"/Script/CoreUObject.Class'/Script/DMXRuntime.DMXEntityFixturePatch'\",EntityId=BC61967946B7385B45A6BC9B7532F0B9)"))
  (:Started
    ;[1 1 1] TurnOn
    (CallFunction|DmxSendFullColor _outfixturepatch "(PortGuid=A0306D4041F169B7B9A915929266279C,bEnabledFlag=True)" (Math|Color|MakeColor (Variables|Default|GetColorBlue) (Variables|Default|GetColorGreen) (Variables|Default|GetColorRed) 255) 1))
  (:Canceled
    ;[1 1 1] TurnOff
    (CallFunction|DmxSendFullColor _outfixturepatch "(PortGuid=A0306D4041F169B7B9A915929266279C,bEnabledFlag=True)" (Math|Color|MakeColor 0 0 0) 1 :!label _label))
  (:Completed
    (goto _label)))

(event Collision|EventActorBeginOverlap
  (params (OtherActor :type Actor%20Object%20Reference)))

(event EventTick
  (params (DeltaSeconds :type Float%20%28single-precision%29)))

(event EventBeginPlay
  (bind _asplayer_controller (Utilities|Casting|CastToPlayerController (Pawn|GetController)))
  (Utilities|IsValid (PlayerController|LocalPlayerSubsystems|GetEnhancedInputLocalPlayerSubsystem _asplayer_controller)
    (:Is%20Valid
      (Input|AddMappingContext (PlayerController|LocalPlayerSubsystems|GetEnhancedInputLocalPlayerSubsystem _asplayer_controller) "/Game/Input/IMC_Dmx.IMC_Dmx" 0 "(bIgnoreAllPressedKeysUntilRelease=True,bForceImmediately=False,bNotifyUserSettings=False)"))))

(fn ConstructionScript)

(fn DmxSendFullColor
  (params (FixturePatch :type DMX%20Entity%20Fixture%20Patch%20Object%20Reference) (DmxOutputPort :type DMX%20Output%20Port%20Reference%20Structure) (Color :type Color%20Structure) (SegmentCount :type Integer) (SegmentIndex :type Integer))
  (bind (_b _g _r) (Math|Color|BreakColor Color))
  (bind _channelmap (LocalVariables|GetChannelMap))
  (bind _parentfixturetypetemplate (Variables|/Script/DMXRuntime.DMXEntityFixturePatch|GetParentFixtureTypeTemplate FixturePatch))
  (bind _modes (Variables|/Script/DMXRuntime.DMXEntityFixtureType|GetModes _parentfixturetypetemplate))
  (bind _output (Utilities|Array|Get(acopy) _modes))
  (bind _channelspan (Utilities|Struct|BreakDMXFixtureMode _output))
  (bind _returnvalue (/ _channelspan SegmentCount))
  (for _index (range (* _returnvalue SegmentIndex) (* _returnvalue (+ SegmentIndex 1)))
    (if (== (Math|Integer|%(Integer) _index 3) 0)
      (LocalVariables|SetChannelVal _r)
      (Utilities|Map|Add _channelmap _index (LocalVariables|GetChannelVal) :!label _label)
      (elif (== (Math|Integer|%(Integer) _index 3) 1)
        (LocalVariables|SetChannelVal _g)
        (goto _label)
        (elif (== (Math|Integer|%(Integer) _index 3) 2)
          (LocalVariables|SetChannelVal _b)
          (goto _label)))))
  (Class|DMXSubsystem|SendDMXtoOutputPort DmxOutputPort _channelmap 1)
  (Development|PrintString "Dmx data sent"))